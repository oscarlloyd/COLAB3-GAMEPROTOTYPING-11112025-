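; BP_JOYMAN is an enemy that trades position-based attacks with the first-person player.
; Normal player hits lower its health and show a talk widget with a random dialogue line; Special hits do nothing.
; AttackPlayer re-rolls AttackChoice at each branch to pick left, special or right, then damages the player according to Currentposition.
; Special and right attacks call OnAttackFinish; left does not, and a failed roll chain does nothing.
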(event `AttackedbyPlayer`
  (params (AttackType :type Name))
  (if (== AttackType "Normal")
    (set `self.JoymanHealth` (- (`self.JoymanHealth`) 10.0))
    (set `self.JoymanTalk` (`|GetArrayItem` (`self.Dialogue`) (`KismetMathLibrary.RandomIntegerInRange` 0 3)))
    (bind _returnvalue (`|CreateWidget` "/Game/UI/WB_JOYMANTALK.WB_JOYMANTALK_C"))
    (bind _output_get (set `self.JoymanTalkRef` _returnvalue))
    (`UserWidget.AddToViewport` _output_get 0)
    (elif (== AttackType "Special")
      _)))

(event `self.ReceiveBeginPlay`
  (set `self.JoymanHealth` 100.0)
  (set `self.JoymanPosition` "Neutral"))

(event `Attack Player`
  (bind _as_bp_first_person_character (`self.As BP First Person Character`))
  (if (== (`KismetArrayLibrary.Array_Random` (`self.AttackChoice`)) 0)
    (`KismetSystemLibrary.PrintString` "JOYMANLeftAttack")
    (bind _asbp_first_person_character (cast `/Game/FirstPerson/Blueprints/BP_FirstPersonCharacter` (`GameplayStatics.GetPlayerCharacter` 0)))
    (set `self.As BP First Person Character` _asbp_first_person_character)
    (if (== (`/Game/FirstPerson/Blueprints/BP_FirstPersonCharacter.Currentposition` _asbp_first_person_character) "Neutral")
      (`KismetSystemLibrary.PrintString` "Hit player" :!label _label)
      (bind _output_get (set `self.DamageDealt` 20.0))
      (`/Game/FirstPerson/Blueprints/BP_FirstPersonCharacter.PlayerGetsHit ` _as_bp_first_person_character _output_get)
      (elif (== (`/Game/FirstPerson/Blueprints/BP_FirstPersonCharacter.Currentposition` _asbp_first_person_character) "Left")
        (goto _label)
        (else
          (`KismetSystemLibrary.PrintString` "MissedPlayer"))))
    (elif (== (`KismetArrayLibrary.Array_Random` (`self.AttackChoice`)) 1)
      (`KismetSystemLibrary.PrintString` "JOYMANSpecialAttack")
      (bind _asbp_first_person_character_2 (cast `/Game/FirstPerson/Blueprints/BP_FirstPersonCharacter` (`GameplayStatics.GetPlayerCharacter` 0)))
      (set `self.As BP First Person Character` _asbp_first_person_character_2)
      (if (== (`/Game/FirstPerson/Blueprints/BP_FirstPersonCharacter.Currentposition` _asbp_first_person_character_2) "Neutral")
        (`KismetSystemLibrary.PrintString` "Hit player" :!label _label_2)
        (bind _output_get_2 (set `self.DamageDealt` 35.0))
        (`/Game/FirstPerson/Blueprints/BP_FirstPersonCharacter.PlayerGetsHit ` _as_bp_first_person_character _output_get_2)
        (elif (== (`/Game/FirstPerson/Blueprints/BP_FirstPersonCharacter.Currentposition` _asbp_first_person_character_2) "Right")
          (goto _label_2)
          (elif (== (`/Game/FirstPerson/Blueprints/BP_FirstPersonCharacter.Currentposition` _asbp_first_person_character_2) "Left")
            (goto _label_2)
            (else
              (`KismetSystemLibrary.PrintString` "MissedPlayer")))))
      (`self.OnAttackFinish`)
      (`KismetSystemLibrary.PrintString` "AttackEND")
      (elif (== (`KismetArrayLibrary.Array_Random` (`self.AttackChoice`)) 2)
        (`KismetSystemLibrary.PrintString` "JOYMANRightAttack")
        (bind _asbp_first_person_character_3 (cast `/Game/FirstPerson/Blueprints/BP_FirstPersonCharacter` (`GameplayStatics.GetPlayerCharacter` 0)))
        (set `self.As BP First Person Character` _asbp_first_person_character_3)
        (if (== (`/Game/FirstPerson/Blueprints/BP_FirstPersonCharacter.Currentposition` _asbp_first_person_character_3) "Neutral")
          (`KismetSystemLibrary.PrintString` "Hit player" :!label _label_3)
          (bind _output_get_3 (set `self.DamageDealt` 20.0))
          (`/Game/FirstPerson/Blueprints/BP_FirstPersonCharacter.PlayerGetsHit ` _as_bp_first_person_character _output_get_3)
          (elif (== (`/Game/FirstPerson/Blueprints/BP_FirstPersonCharacter.Currentposition` _asbp_first_person_character_3) "Right")
            (goto _label_3)
            (else
              (`KismetSystemLibrary.PrintString` "MissedPlayer"))))
        (`self.OnAttackFinish`)
        (`KismetSystemLibrary.PrintString` "AttackEND")))))

(fn `UserConstructionScript`)